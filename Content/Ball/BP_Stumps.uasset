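; Cricket stumps actor that breaks apart when a component tagged "ball" overlaps its box trigger.
; Physics simulation is enabled on Gills, Gills1 and Stumps, and an impulse is applied to them plus Stumps1 and Stumps2.
; It adds an existing Out widget to the viewport, or only creates one if none exists.
; After a short delay it opens the Ground level.
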(event `self.Box.OnComponentBeginOverlap`
  (params (OverlappedComponent :type "PrimitiveComponent Object Reference") (OtherActor :type "Actor Object Reference") (OtherComp :type "PrimitiveComponent Object Reference") (OtherBodyIndex :type Integer) (bFromSweep :type Boolean) (SweepResult :type "HitResult Structure (by ref)"))
  (if (`ActorComponent.ComponentHasTag` OtherComp "ball")
    (`PrimitiveComponent.SetSimulatePhysics` (`self.Gills`) true)
    (`PrimitiveComponent.SetSimulatePhysics` (`self.Stumps`) true)
    (`PrimitiveComponent.SetSimulatePhysics` (`self.Gills1`) true)
    (`PrimitiveComponent.AddImpulse` (`self.Stumps1`) (100.0 0.0 100.0) "None" false)
    (`PrimitiveComponent.AddImpulse` (`self.Stumps2`) (100.0 0.0 100.0) "None" false)
    (`PrimitiveComponent.AddImpulse` (`self.Gills`) (100.0 0.0 100.0) "None" false)
    (`PrimitiveComponent.AddImpulse` (`self.Gills1`) (100.0 0.0 100.0) "None" false)
    (`PrimitiveComponent.AddImpulse` (`self.Stumps`) (100.0 0.0 100.0) "None" false)
    (bind _outwidget (`self.OutWidget`)
      (:`then`
        (`UserWidget.AddToViewport` _outwidget 0))
      (:`else`
        (bind _returnvalue (`|CreateWidget` "/Game/ui/Out.Out_C"))
        (set `self.OutWidget` _returnvalue)))
    (`KismetSystemLibrary.Delay` 2.0)
    (`GameplayStatics.OpenLevelBySoftObjectPtr` "/Game/Ground.Ground")))

(fn `UserConstructionScript`)