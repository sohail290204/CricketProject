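; Cricket ball actor that detects the outcome of a delivery and scores runs.
; Sphere overlaps with tagged zones award singles, twos, fours or sixes on bat hits, using a looping trace timer to detect bounces that separate fours from sixes.
; Runs update the game mode and bowler (BP_Enemy), show a popup and cheer each fifty.
; Scoring, unhit wides or a stopped ball reset bowling and destroy the ball.
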(event `self.ReceiveBeginPlay`
  (bind _asbp_cricket_player (cast `/Game/Player/BP/BP_CricketPlayer` (`GameplayStatics.GetPlayerCharacter` 0)))
  (set `self.As BP Cricket Player` _asbp_cricket_player)
  (bind _ascricketgamemode (cast `/Game/Player/CRICKETGAMEMODE` (`GameplayStatics.GetGameMode`)))
  (set `self.As CRICKETGAMEMODE` _ascricketgamemode))

(event `Short`
  ; Tappa check
  (`KismetSystemLibrary.K2_SetTimerDelegate` (delegate `CustomEvent`) 0.1 true))

(event `CustomEvent`
  (bind _returnvalue (`SceneComponent.K2_GetComponentLocation` (`self.untitled`)))
  ; Tappa check
  (if (`self.HitBat`)
    (bind _outhit (`KismetSystemLibrary.SphereTraceSingle` _returnvalue _returnvalue 20.0 "TraceTypeQuery1"))
    (if (`GameplayStatics.BreakHitResult` _outhit)
      (set `self.TappaTrue?` true))))

(event `self.ReceiveTick`
  (params (DeltaSeconds :type "Float (single-precision)"))
  ; Velocity check
  (`|ExecutionSequence`
    (:`then_0`
      (`KismetSystemLibrary.Delay` 1.0)
      (if (<= (`KismetMathLibrary.VSize` (`SceneComponent.GetComponentVelocity` (`self.untitled`))) 0.0)
        (`self.BallVelocityCheck`)))
    (:`then_1`
      (`/Engine/EditorBlueprintResources/StandardMacros.DoOnce` false
        (:`Completed`
          (bind _returnvalue (`GameplayStatics.GetActorOfClass` "/Game/Player/NewFolder/BP_Enemy.BP_Enemy_C"))
          (set `self.Enemy` _returnvalue))))))

(event `ResetDoonce`
  ; 6 4 Boundry chcek
  (`/Engine/EditorBlueprintResources/StandardMacros.DoOnce` false :!via `Reset`
    (:`Completed`
      (bind _run (`self.Run`)
        (:`then`
          (`UserWidget.AddToViewport` _run 0))
        (:`else`
          (bind _returnvalue (`|CreateWidget` "/Game/ui/Run.Run_C"))
          (bind _output_get (set `self.Run` _returnvalue))
          (`UserWidget.AddToViewport` _output_get 0)))
      (`TextBlock.SetText` (`/Game/ui/Run.Run` _output_get) (`self.In Tool Tip Text`))
      (`KismetSystemLibrary.Delay` 0.2)
      (set `self.In Tool Tip Text` "")
      (`|ExecutionSequence`
        (:`then_0`
          (`self.Enemy`
            (:`then`
              (`/Game/Player/NewFolder/BP_Enemy.ResetBawling`)
              (`KismetSystemLibrary.Delay` 1.0)
              (bind _run_2 (`self.Run`)
                (:`then`
                  (`Widget.RemoveFromParent` _run_2)
                  (`KismetSystemLibrary.Delay` 0.2))
                (:`else`
                  _))
              (`self.K2_DestroyActor`))
            (:`else`)))
        (:`then_1`
          (`self.ResetDoonce`))))))

(event `Check Celebration`
  (bind _as_cricketgamemode (`self.As CRICKETGAMEMODE`))
  (bind _returnvalue (+ (`/Game/Player/CRICKETGAMEMODE.lastCelebratedScore` _as_cricketgamemode) 50))
  (if (<= _returnvalue (`/Game/Player/CRICKETGAMEMODE.Score` _as_cricketgamemode))
    (set `/Game/Player/CRICKETGAMEMODE.lastCelebratedScore` _returnvalue _as_cricketgamemode)
    (`/Game/Player/BP/BP_CricketPlayer.PlayCrowdCheer` (`self.As BP Cricket Player`))))

(event `PlaySound`)

(event `self.Sphere.OnComponentBeginOverlap`
  (params (OverlappedComponent :type "PrimitiveComponent Object Reference") (OtherActor :type "Actor Object Reference") (OtherComp :type "PrimitiveComponent Object Reference") (OtherBodyIndex :type Integer) (bFromSweep :type Boolean) (SweepResult :type "HitResult Structure (by ref)"))
  (bind _as_cricketgamemode (`self.As CRICKETGAMEMODE`))
  (bind _enemy (`self.Enemy`))
  (bind _enemy_2 (`self.Enemy`))
  (bind _ballcount (`/Game/Player/NewFolder/BP_Enemy.BallCount` _enemy))
  (bind _runsperball (`/Game/Player/NewFolder/BP_Enemy.RunsPerBall` _enemy))
  (bind _ballcount_2 (`/Game/Player/NewFolder/BP_Enemy.BallCount` _enemy_2))
  (bind _runsperball_2 (`/Game/Player/NewFolder/BP_Enemy.RunsPerBall` _enemy_2))
  (bind _as_bp_cricket_player (`self.As BP Cricket Player`)
    (:`then`
      (if (`/Game/Player/BP/BP_CricketPlayer.Out` _as_bp_cricket_player)
        _
        (elif (`ActorComponent.ComponentHasTag` OtherComp "Boundry")
          (if (`self.HitBat`)
            (if (`self.TappaTrue?`)
              (set `self.In Tool Tip Text` "Four")
              (`self.PlaySound`)
              (bind _as_cricketgamemode_2 (`self.As CRICKETGAMEMODE`)
                (:`then`
                  (set `/Game/Player/CRICKETGAMEMODE.Score` (+ (`/Game/Player/CRICKETGAMEMODE.Score` _as_cricketgamemode_2) 4) _as_cricketgamemode_2)
                  (`BlueprintMapLibrary.Map_Add` _runsperball_2 "4" _ballcount_2)
                  (`/Game/Player/CRICKETGAMEMODE.Add Balls` _as_cricketgamemode "4"))
                (:`else`))
              (else
                (set `self.In Tool Tip Text` "Six")
                (`self.PlaySound`)
                (bind _as_cricketgamemode_3 (`self.As CRICKETGAMEMODE`)
                  (:`then`
                    (set `/Game/Player/CRICKETGAMEMODE.Score` (+ (`/Game/Player/CRICKETGAMEMODE.Score` _as_cricketgamemode_3) 6) _as_cricketgamemode_3)
                    (`BlueprintMapLibrary.Map_Add` _runsperball_2 "6" _ballcount_2)
                    (`/Game/Player/CRICKETGAMEMODE.Add Balls` _as_cricketgamemode "6"))
                  (:`else`))))
            (`self.Create Widget and SetBoundryRun`))
          (elif (`ActorComponent.ComponentHasTag` OtherComp "back")
            (`PrimitiveComponent.SetSimulatePhysics` (`self.untitled`) false)
            (if (`/Game/Player/BP/BP_CricketPlayer.WideTrue` (`self.As BP Cricket Player`))
              _
              (elif (`self.HitBat`)
                (set `self.In Tool Tip Text` "One")
                (bind _as_cricketgamemode_4 (`self.As CRICKETGAMEMODE`)
                  (:`then`
                    (set `/Game/Player/CRICKETGAMEMODE.Score` (+ (`/Game/Player/CRICKETGAMEMODE.Score` _as_cricketgamemode_4) 1) _as_cricketgamemode_4)
                    (`BlueprintMapLibrary.Map_Add` _runsperball "1" _ballcount)
                    (`/Game/Player/CRICKETGAMEMODE.Add Balls` (`self.As CRICKETGAMEMODE`) "1")
                    (`self.Create Widget and SetBoundryRun`))
                  (:`else`))))
            (elif (`ActorComponent.ComponentHasTag` OtherComp "Right")
              (`PrimitiveComponent.SetSimulatePhysics` (`self.untitled`) false)
              (if (`self.HitBat`)
                (set `self.In Tool Tip Text` "Two")
                (bind _as_cricketgamemode_5 (`self.As CRICKETGAMEMODE`)
                  (:`then`
                    (set `/Game/Player/CRICKETGAMEMODE.Score` (+ (`/Game/Player/CRICKETGAMEMODE.Score` _as_cricketgamemode_5) 2) _as_cricketgamemode_5)
                    (`BlueprintMapLibrary.Map_Add` _runsperball "2" _ballcount)
                    (`/Game/Player/CRICKETGAMEMODE.Add Balls` (`self.As CRICKETGAMEMODE`) "2")
                    (`self.Create Widget and SetBoundryRun`))
                  (:`else`)))
              (elif (`ActorComponent.ComponentHasTag` OtherComp "wide")
                (if (not (`self.HitBat`))
                  (bind _enemy_3 (`self.Enemy`)
                    (:`then`
                      (`/Game/Player/NewFolder/BP_Enemy.ResetBawling` _enemy_3)
                      (`KismetSystemLibrary.Delay` 0.2)
                      (`self.K2_DestroyActor`))
                    (:`else`)))))))))
    (:`else`)))

(event `BallVelocityCheck`
  (bind _enemy (`self.Enemy` :!label _label)
    (:`then`
      (`/Game/Player/NewFolder/BP_Enemy.ResetBawling` _enemy)
      (`KismetSystemLibrary.Delay` 2.0)
      (bind _run (`self.Run`)
        (:`then`
          (`Widget.RemoveFromParent` _run)
          (`KismetSystemLibrary.Delay` 0.2))
        (:`else`
          _))
      (`self.K2_DestroyActor`))
    (:`else`)))

(event `Create Widget and SetBoundryRun`
  (set `/Game/Player/NewFolder/BP_Enemy.RunInBall` true (`self.Enemy`))
  (`self.Check Celebration`)
  (`PrimitiveComponent.SetSimulatePhysics` (`self.untitled`) false)
  (bind _run (`self.Run`)
    (:`then`
      (`UserWidget.AddToViewport` _run 0))
    (:`else`
      (bind _returnvalue (`|CreateWidget` "/Game/ui/Run.Run_C"))
      (bind _output_get (set `self.Run` _returnvalue))
      (`UserWidget.AddToViewport` _output_get 0)))
  (`TextBlock.SetText` (`/Game/ui/Run.Run` (`self.Run`)) (`self.In Tool Tip Text`))
  (`KismetSystemLibrary.Delay` 0.2)
  (set `self.In Tool Tip Text` "")
  (goto _label))

(fn `UserConstructionScript`)