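; BP_Enemy is the AI bowler in a cricket game, bowling repeatedly at the player.
; Each cycle picks one of two bowling points and a random marked bounce spot, plays the bowling animation, and briefly enables the player's Allow flag.
; A looping timer drives the run-up, then a ball spawns at Arrow1 with a random-strength impulse toward the spot.
; After a delay, it destroys ball and marker, clears the player's hit flag and restarts.
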(event `self.ReceiveBeginPlay`
  (`|ExecutionSequence`
    (:`then_0`
      (`KismetSystemLibrary.Delay` 2.0)
      (set `/Game/Player/BP/BP_CricketPlayer.Allow` true (stale `self.ReceiveBeginPlay` _asbp_cricket_player) :!label _label)
      (`|ExecutionSequence`
        (:`then_0`
          (`SkeletalMeshComponent.PlayAnimation` (`self.Mesh`) "/Game/Player/NewFolder/Bowlinf_Anim.Bowlinf_Anim" false)
          (`|ExecutionSequence`
            (:`then_0`
              (bind _returnvalue (`KismetSystemLibrary.K2_SetTimerDelegate` (delegate `CustomEvent`) 0.01 true)))
            (:`then_1`
              (`KismetSystemLibrary.Delay` 2.0)
              (set `/Game/Player/BP/BP_CricketPlayer.Allow` false (stale `self.ReceiveBeginPlay` _asbp_cricket_player)))))
        (:`then_1`
          (`self.K2_SetActorLocation` (select `bool` (`KismetMathLibrary.RandomBool`) :`false` (`self.BowlingPoint2`) :`true` (`self.BowlingPoint2_0`)))
          (bind _output_get (set `self.BounceLocationPoint` (`|GetArrayItem` (`self.BounceLocation`) (`KismetMathLibrary.RandomIntegerInRange` 0 16))))
          (bind _returnvalue_2 (`|SpawnActorFromClass` "/Game/Ball/BP_SpotPoint.BP_SpotPoint_C" (`KismetMathLibrary.MakeTransform` _output_get) "AlwaysSpawn" "MultiplyWithRoot" null null)))))
    (:`then_1`
      (bind _asbp_cricket_player (cast `/Game/Player/BP/BP_CricketPlayer` (`GameplayStatics.GetPlayerCharacter` 0)))
      (set `/Game/Player/BP/BP_CricketPlayer.Allow` true _asbp_cricket_player))))

(event `CustomEvent`
  (bind (_returnvalue_location _returnvalue_rotation) (`KismetMathLibrary.BreakTransform` (`SceneComponent.K2_GetComponentToWorld` (`self.Arrow1`))))
  (`|ExecutionSequence`
    (:`then_0`
      (`self.AddMovementInput` (1.0 0.0 0.0)))
    (:`then_1`
      (`KismetSystemLibrary.Delay` 2.0)
      (`KismetSystemLibrary.K2_PauseTimerHandle` (stale `self.ReceiveBeginPlay` _returnvalue))
      (bind _returnvalue (`|SpawnActorFromClass` "/Game/Ball/BP_Ball.BP_Ball_C" (`KismetMathLibrary.MakeTransform` _returnvalue_location _returnvalue_rotation (0.1 0.1 0.1)) "AlwaysSpawn" "MultiplyWithRoot" null null))
      (`PrimitiveComponent.AddImpulse` (`/Game/Ball/BP_Ball.untitled` _returnvalue) (* (`KismetMathLibrary.Normal` (- (`self.BounceLocationPoint`) _returnvalue_location)) (`KismetMathLibrary.RandomIntegerInRange` 4000 5000)) "None" false)
      (`KismetSystemLibrary.Delay` 5.0)
      (`self.K2_DestroyActor` _returnvalue)
      (set `/Game/Player/BP/BP_CricketPlayer.BallHitTrue` false (stale `self.ReceiveBeginPlay` _asbp_cricket_player))
      (`self.ResetBawling`))))

(event `ResetBawling`
  (`self.K2_DestroyActor` (stale `self.ReceiveBeginPlay` _returnvalue_2))
  (goto _label))

(fn `UserConstructionScript`)